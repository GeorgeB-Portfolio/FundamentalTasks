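; BP_Rifle is a rifle pickup Blueprint with prototype equip detection that only prints debug messages.
; A sphere's begin and end overlaps track whether a BP_Player is in range, storing the player reference on entry.
; Both overlaps call the try-equip event, which checks the player's EquipPressed flag only while overlapping.
; The flag is read at that moment rather than polled, and no attachment happens.
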(event `TryEquip_Event`
  (if (`self.OverlappingPlayer`)
    (if (`/Game/Blueprints/BP_Player.EquipPressed` (`self.PlayerReference`))
      (`KismetSystemLibrary.PrintString` "Equipped")
      (else
        (`KismetSystemLibrary.PrintString` "Not equiped")))))

(event `self.Sphere.OnComponentBeginOverlap`
  (params (OverlappedComponent :type "PrimitiveComponent Object Reference") (OtherActor :type "Actor Object Reference") (OtherComp :type "PrimitiveComponent Object Reference") (OtherBodyIndex :type Integer) (bFromSweep :type Boolean) (SweepResult :type "HitResult Structure (by ref)"))
  (bind _asbp_player (cast `/Game/Blueprints/BP_Player` OtherActor)
    (:`then`
      (set `self.PlayerReference` _asbp_player)
      (set `self.OverlappingPlayer` true)
      (`self.TryEquip_Event`))
    (:`CastFailed`
      (`KismetSystemLibrary.PrintString` "Cast Failed"))))

(event `self.Sphere.OnComponentEndOverlap`
  (params (OverlappedComponent :type "PrimitiveComponent Object Reference") (OtherActor :type "Actor Object Reference") (OtherComp :type "PrimitiveComponent Object Reference") (OtherBodyIndex :type Integer))
  (cast `/Game/Blueprints/BP_Player` OtherActor)
  (set `self.OverlappingPlayer` false)
  (`self.TryEquip_Event`))

(fn `UserConstructionScript`)