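; BP_Follower is an actor that trails the player at a fixed offset.
; On BeginPlay it finds and caches the BP_Player actor.
; Each Tick it places itself behind the player capsule's forward vector and below the player's location, with no interpolation or sweep.
; The world-space result is applied through SetActorRelativeLocation, so it matches world position only while the follower has no transformed parent.
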(event `self.ReceiveBeginPlay`
  (bind _returnvalue (`GameplayStatics.GetActorOfClass` "/Game/Blueprints/BP_Player.BP_Player_C"))
  (set `self.PlayerRef` _returnvalue))

(event `self.ReceiveTick`
  (params (DeltaSeconds :type "Float (single-precision)"))
  (bind _playerref (`self.PlayerRef`))
  (bind (_returnvalue_x _returnvalue_y _returnvalue_z) (`KismetMathLibrary.BreakVector` (`self.K2_GetActorLocation` _playerref)))
  (`self.K2_SetActorRelativeLocation` (+ (* (`SceneComponent.GetForwardVector` (`Character.CapsuleComponent` _playerref)) -200.0) (`KismetMathLibrary.MakeVector` _returnvalue_x _returnvalue_y (- _returnvalue_z 60.0)))))

(fn `UserConstructionScript`)