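; BP_Key is a key pickup actor that registers itself with the player while they stand inside its Box trigger.
; Box overlap stores the BP_Player and sets that player's KeyRef to this key, then clears it on exit only if it still points here.
; Equip_Event sets KeyObtained on the key and immediately destroys the actor.
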(event `Equip_Event`
  (set `self.KeyObtained` true)
  (`self.K2_DestroyActor`))

(event `self.Box.OnComponentBeginOverlap`
  (params (OverlappedComponent :type "PrimitiveComponent Object Reference") (OtherActor :type "Actor Object Reference") (OtherComp :type "PrimitiveComponent Object Reference") (OtherBodyIndex :type Integer) (bFromSweep :type Boolean) (SweepResult :type "HitResult Structure (by ref)"))
  (bind _asbp_player (cast `/Game/Blueprints/BP_Player` OtherActor)
    (:`then`
      (bind _output_get (set `self.PlayerReference` _asbp_player))
      (set `/Game/Blueprints/BP_Player.KeyRef` self _output_get))
    (:`CastFailed`
      (`KismetSystemLibrary.PrintString` "Cast Failed"))))

(event `self.Box.OnComponentEndOverlap`
  (params (OverlappedComponent :type "PrimitiveComponent Object Reference") (OtherActor :type "Actor Object Reference") (OtherComp :type "PrimitiveComponent Object Reference") (OtherBodyIndex :type Integer))
  (bind _playerreference (`self.PlayerReference`))
  (cast `/Game/Blueprints/BP_Player` OtherActor)
  (if (== (`/Game/Blueprints/BP_Player.KeyRef` _playerreference) self)
    (set `/Game/Blueprints/BP_Player.KeyRef` null _playerreference)))

(fn `UserConstructionScript`)