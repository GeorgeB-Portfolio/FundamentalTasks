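; Player character Blueprint handling movement, look, jump, dash, shooting, a fireball spell and Equip interactions.
; Dash launches the character forward then upward, with a looping timer counting down its cooldown and updating the BasicUI widget created at BeginPlay.
; Equip acts on whichever key, gun or button references are valid, and Shoot calls OnFire.
; Fireballs spawn ahead along the camera rotation, while the F key directly subtracts Health.
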(event `self.ReceiveBeginPlay`
  (bind _returnvalue (`|CreateWidget` "/Game/UI/BasicUI.BasicUI_C"))
  (bind _output_get (set `self.UI` _returnvalue))
  (`UserWidget.AddToViewport` _output_get 0))

(event `InputAction|Dash`
  (params (Key :type "Key Structure"))
  (bind _returnvalue (`self.K2_GetActorRotation`))
  (:`Pressed`
    (if (== (`self.DashCooldown`) 0.0)
      (`self.LaunchCharacter` (* (`KismetMathLibrary.GetForwardVector` _returnvalue) 500.0))
      (`KismetSystemLibrary.Delay` 0.01)
      (`self.LaunchCharacter` (* (`KismetMathLibrary.GetUpVector` _returnvalue) 100.0))
      (bind _returnvalue_2 (`KismetSystemLibrary.K2_SetTimerDelegate` (delegate `ReduceDashCooldown`) (`GameplayStatics.GetWorldDeltaSeconds`) true))
      (set `self.DashTimer` _returnvalue_2)
      (`/Game/UI/BasicUI.DashCooldown` (`self.UI`))
      (set `self.DashCooldown` 1.0))))

(event `InputAxis|Forward/Back`
  (params (AxisValue :type "Float (single-precision)"))
  (`self.Move Forward` AxisValue))

(event `InputAxis|Left/Right`
  (params (AxisValue :type "Float (single-precision)"))
  (`self.MoveRight` AxisValue))

(event `ReduceDashCooldown`
  (bind _output_get (set `self.DashCooldown` (`KismetMathLibrary.FClamp` (- (`self.DashCooldown`) (`GameplayStatics.GetWorldDeltaSeconds`)))))
  (`/Game/UI/BasicUI.ReduceDashCooldown` (`self.UI`) _output_get)
  (if (== (`self.DashCooldown`) 0.0)
    (`KismetSystemLibrary.K2_ClearAndInvalidateTimerHandle` (`self.DashTimer`))))

(event `InputAction|Jump`
  (params (Key :type "Key Structure"))
  (:`Pressed`
    (`self.Jump`)))

(event `InputAxis|LookUp/Down`
  (params (AxisValue :type "Float (single-precision)"))
  (`self.AddControllerPitchInput` AxisValue))

(event `Key|F`
  (params (Key :type "Key Structure"))
  (:`Pressed`
    (set `self.Health` (- (`self.Health`) 25.0))))

(event `InputAxis|Turning`
  (params (AxisValue :type "Float (single-precision)"))
  (`self.AddControllerYawInput` AxisValue))

(event `InputAction|Equip`
  (params (Key :type "Key Structure"))
  (bind _keyref (`self.KeyRef`))
  (:`Pressed`
    (`/Engine/EditorBlueprintResources/StandardMacros.IsValid` _keyref
      (:`Is Valid`
        (`/Game/Blueprints/BP_Key.Equip_Event` _keyref)
        (set `self.KeyEquipped` true)))))

(event `InputAction|Equip`
  (params (Key :type "Key Structure"))
  (:`Pressed`
    (`/Engine/EditorBlueprintResources/StandardMacros.IsValid` (`self.GunRef`)
      (:`Is Valid`
        (`/Game/Blueprints/BP_Rifle.Equip_Event` (`self.GunRef`))))))

(event `InputAction|Shoot`
  (params (Key :type "Key Structure"))
  (:`Pressed`
    (`self.OnFire`)))

(event `InputAction|Spell 1`
  (params (Key :type "Key Structure"))
  (bind _returnvalue (`PlayerCameraManager.GetCameraRotation` (`GameplayStatics.GetPlayerCameraManager` 0)))
  (:`Pressed`
    (`|SpawnActorFromClass` "/Game/Blueprints/BP_Spell_Fireball.BP_Spell_Fireball_C" (`KismetMathLibrary.MakeTransform` (+ (`self.K2_GetActorLocation`) (`KismetMathLibrary.GreaterGreater_VectorRotator` (100.0 0.0 0.0) _returnvalue)) _returnvalue) "Undefined" "OverrideRootScale" null true null)))

(event `InputAction|Equip`
  (params (Key :type "Key Structure"))
  (:`Pressed`
    (`/Engine/EditorBlueprintResources/StandardMacros.IsValid` (`self.ButtonRef`)
      (:`Is Valid`
        (`/Game/Blueprints/BP_Reset_Button.Button_Press` (`self.ButtonRef`))))))

(fn `Move Forward`
  (params (AxisValue :type "Float (double-precision)"))
  (bind (_returnvalue_roll _returnvalue_pitch _returnvalue_yaw) (`KismetMathLibrary.BreakRotator` (`self.GetControlRotation`)))
  (`self.AddMovementInput` (`KismetMathLibrary.GetForwardVector` (`KismetMathLibrary.MakeRotator` 0.0 0.0 _returnvalue_yaw)) AxisValue))

(fn `MoveRight`
  (params (`Axis Value` :type "Float (double-precision)"))
  (bind (_returnvalue_roll _returnvalue_pitch _returnvalue_yaw) (`KismetMathLibrary.BreakRotator` (`self.GetControlRotation`)))
  (`self.AddMovementInput` (`KismetMathLibrary.GetRightVector` (`KismetMathLibrary.MakeRotator` 0.0 0.0 _returnvalue_yaw)) `Axis Value`))

(fn `UserConstructionScript`)